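; BP_TargetMover drives a shooting course target, drifting it around the mover's location while the course is active.
; A self-repeating event picks a random horizontal and vertical offset after each random delay.
; Tick interpolates the Target toward that offset and turns it to face the course initiator's first-person camera.
; The construction script centers the mover on the referenced course in X and Y, keeping its own height.
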(event `self.ReceiveBeginPlay`
  ;[0 0 0] Target Movement
  ;;[1 1 1] Reposition offset location
  (`self.Reposition`))

(event `Reposition`
  (bind _range (`self.Range`))
  (bind _range_2 (`self.Range`))
  ;[0 0 0] Target Movement
  ;;[1 1 1] Reposition offset location
  (set `self.RandomOffsetLocation` (`KismetMathLibrary.MakeVector` (`KismetMathLibrary.RandomFloatInRange` (* _range -1.0) _range) (`KismetMathLibrary.RandomFloatInRange` (* _range_2 -1.0) _range_2) (`KismetMathLibrary.RandomFloatInRange` 100.0 (`self.VerticalRange`))))
  ;;[1 1 1] Reposition after delay
  (`KismetSystemLibrary.Delay` (`KismetMathLibrary.RandomFloatInRange` 0.0 (`self.SetOffsetDelayRange`)))
  (`self.Reposition`))

(event `self.ReceiveTick`
  (params (DeltaSeconds :type "Float (single-precision)"))
  (bind _courseinitiatorcharacter (`/Game/FPSK/Blueprint/CourseLogic/BP_CourseVolume.CourseInitiatorCharacter` (`self.CourseReference`)))
  ;[0 0 0] Target Movement
  ;;[1 1 1] Only if course reference is valid and course is active
  (`/Engine/EditorBlueprintResources/StandardMacros.IsValid` _courseinitiatorcharacter
    (:`Is Valid`
      (if (`/Game/FPSK/Blueprint/CourseLogic/BP_CourseVolume.CourseRuntimeActive` (`self.CourseReference`))
        ;;[1 1 1] Smoothly move target to randomized location and rotate toward course initiator camera
        (`self.K2_SetActorTransform` (`self.Target`) (`KismetMathLibrary.MakeTransform` (`KismetMathLibrary.VInterpTo` (`self.K2_GetActorLocation` (`self.Target`)) (+ (`self.K2_GetActorLocation`) (`self.RandomOffsetLocation`)) (`GameplayStatics.GetWorldDeltaSeconds`) (`self.MovementSpeed`)) (`KismetMathLibrary.FindLookAtRotation` (`self.K2_GetActorLocation` (`self.Target`)) (`SceneComponent.K2_GetComponentLocation` (`/Game/FPSK/FirstPersonAssets/FirstPersonBP/Blueprints/FirstPersonCharacter.FirstPersonCamera` _courseinitiatorcharacter)))) false false)))))

(fn `UserConstructionScript`
  ;[0 0 0] Center to course reference
  (`/Engine/EditorBlueprintResources/StandardMacros.IsValid` (`self.CourseReference`)
    (:`Is Valid`
      (`self.K2_SetActorLocation` (`KismetMathLibrary.MakeVector` (.x (`self.K2_GetActorLocation` (`self.CourseReference`))) (.y (`self.K2_GetActorLocation` (`self.CourseReference`))) (.z (`self.K2_GetActorLocation`)))))))