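; Modular room Blueprint that builds a four-sided room piece in its construction script from per-instance options.
; Toggles add static mesh components for each wall, floor and roof at offsets from the wall center offset and roof height, then assign their meshes.
; Index arrays place corner beams, scaled to height, and rotated roof frames as instanced static meshes.
; A final AlignTool call aligns the piece against a reference in the editor.
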(fn `UserConstructionScript`
  (bind _roof (`self.Roof`))
  (bind _wallcenteroffset (`self.WallCenterOffset`))
  (bind _wallcenteroffset_2 (`self.WallCenterOffset`))
  (bind _wallcenteroffset_3 (`self.WallCenterOffset`))
  (bind _floor (`self.Floor`))
  (bind _wallcenteroffset_4 (`self.WallCenterOffset`))
  (bind _rightwall (`self.RightWall`))
  (bind _frontwall (`self.FrontWall`))
  (bind _backwall (`self.BackWall`))
  (bind _leftwall (`self.LeftWall`))
  (bind _returnvalue (* (`self.WallCenterOffset`) -1.0))
  (bind _returnvalue_2 (* (`self.WallCenterOffset`) -1.0))
  (`|ExecutionSequence`
    (:`then_0`
      ;[0 0 0] Construct walls
      (`|ExecutionSequence`
        (:`then_0`
          (if (`self.ConstructFrontWall`)
            (bind _returnvalue_3 (`AddComponent|NODE_AddStaticMeshComponent-0` :`RelativeTransform` (`KismetMathLibrary.MakeTransform` (`KismetMathLibrary.MakeVector` 0.0 (`self.WallCenterOffset`)))))
            (set `self.FrontWall` _returnvalue_3)))
        (:`then_1`
          (if (`self.ConstructBackWall`)
            (bind _returnvalue_4 (`AddComponent|NODE_AddStaticMeshComponent-1` :`RelativeTransform` (`KismetMathLibrary.MakeTransform` (`KismetMathLibrary.MakeVector` 0.0 (* (`self.WallCenterOffset`) -1.0)) (struct :`Pitch` 180.0 :`Yaw` 180.0 :`Roll` 180.0))))
            (set `self.BackWall` _returnvalue_4)))
        (:`then_2`
          (if (`self.ConstructLeftWall`)
            (bind _returnvalue_5 (`AddComponent|NODE_AddStaticMeshComponent-3` :`RelativeTransform` (`KismetMathLibrary.MakeTransform` (`KismetMathLibrary.MakeVector` (* (`self.WallCenterOffset`) -1.0)) (struct :`Yaw` -90.0))))
            (set `self.LeftWall` _returnvalue_5)))
        (:`then_3`
          (if (`self.ConstructRightWall`)
            (bind _returnvalue_6 (`AddComponent|NODE_AddStaticMeshComponent-2` :`RelativeTransform` (`KismetMathLibrary.MakeTransform` (`KismetMathLibrary.MakeVector` (`self.WallCenterOffset`)) (struct :`Yaw` 90.0))))
            (set `self.RightWall` _returnvalue_6)))
        (:`then_4`
          (if (`self.ConstructFloor`)
            (bind _returnvalue_7 (`AddComponent|NODE_AddStaticMeshComponent-5`))
            (set `self.Floor` _returnvalue_7)))
        (:`then_5`
          (if (`self.ConstructRoof`)
            (bind _returnvalue_8 (`AddComponent|NODE_AddStaticMeshComponent-4` :`RelativeTransform` (`KismetMathLibrary.MakeTransform` (`KismetMathLibrary.MakeVector` 0.0 0.0 (`self.RoofHeight`)))))
            (set `self.Roof` _returnvalue_8)))))
    (:`then_1`
      ;[0 0 0] Set mesh for each panel
      (`|ExecutionSequence`
        (:`then_0`
          (`/Engine/EditorBlueprintResources/StandardMacros.IsValid` _frontwall
            (:`Is Valid`
              (`StaticMeshComponent.SetStaticMesh` _frontwall (`self.FrontWallMesh`)))))
        (:`then_1`
          (`/Engine/EditorBlueprintResources/StandardMacros.IsValid` _backwall
            (:`Is Valid`
              (`StaticMeshComponent.SetStaticMesh` _backwall (`self.BackWallMesh`)))))
        (:`then_2`
          (`/Engine/EditorBlueprintResources/StandardMacros.IsValid` _leftwall
            (:`Is Valid`
              (`StaticMeshComponent.SetStaticMesh` _leftwall (`self.LeftWallMesh`)))))
        (:`then_3`
          (`/Engine/EditorBlueprintResources/StandardMacros.IsValid` _rightwall
            (:`Is Valid`
              (`StaticMeshComponent.SetStaticMesh` _rightwall (`self.RightWallMesh`)))))
        (:`then_4`
          (`/Engine/EditorBlueprintResources/StandardMacros.IsValid` _roof
            (:`Is Valid`
              (`StaticMeshComponent.SetStaticMesh` _roof (`self.RoofMesh`)))))
        (:`then_5`
          (`/Engine/EditorBlueprintResources/StandardMacros.IsValid` _floor
            (:`Is Valid`
              (`StaticMeshComponent.SetStaticMesh` _floor (`self.FloorMesh`)))))))
    (:`then_2`
      ;[0 0 0] Construct Support Beams
      ;;[1 1 1] Create instanced static mesh component if there are beams in array
      (if (> (`KismetArrayLibrary.Array_Length` (`self.CornerBeams`)) 0)
        (bind _returnvalue_9 (`AddComponent|NODE_AddInstancedStaticMeshComponent-0`))
        (set `self.BeamMeshInstances` _returnvalue_9)
        ;;[1 1 1] Add beam and move to corner based on index
        (for _array_element (`self.CornerBeams`)
          (`InstancedStaticMeshComponent.AddInstance` (`self.BeamMeshInstances`) (`KismetMathLibrary.MakeTransform` (select `int` _array_element :`0` (`KismetMathLibrary.MakeVector` _wallcenteroffset _wallcenteroffset) :`1` (`KismetMathLibrary.MakeVector` _wallcenteroffset_2 (* _wallcenteroffset_2 -1.0)) :`2` (`KismetMathLibrary.MakeVector` (* _wallcenteroffset_3 -1.0) _wallcenteroffset_3) :`3` (`KismetMathLibrary.MakeVector` _returnvalue _returnvalue)) (struct) (`KismetMathLibrary.MakeVector` 1.0 1.0 (`self.SupportBeamHeight`)))))))
    (:`then_3`
      ;[0 0 0] Construct Roof Frames
      ;;[1 1 1] Create instanced static mesh component if there are roof frames in array
      (if (> (`KismetArrayLibrary.Array_Length` (`self.RoofFrames`)) 0)
        (bind _returnvalue_10 (`AddComponent|NODE_AddInstancedStaticMeshComponent-1`))
        (set `self.RoofFrameMeshes` _returnvalue_10)
        ;;[1 1 1] Add roof frame instance and rotate based on index
        (for _array_element_2 (`self.RoofFrames`)
          (`InstancedStaticMeshComponent.AddInstance` (`self.RoofFrameMeshes`) (`KismetMathLibrary.MakeTransform` (`KismetMathLibrary.MakeVector` (select `int` _array_element_2 :`0` 0.0 :`1` _wallcenteroffset_4 :`2` 0.0 :`3` _returnvalue_2) (select `int` _array_element_2 :`0` _wallcenteroffset_4 :`1` 0.0 :`2` _returnvalue_2 :`3` 0.0) (`self.RoofHeight`)) (`KismetMathLibrary.MakeRotator` 0.0 0.0 (* _array_element_2 90.0)))))))
    (:`then_4`
      ;[0 0 0] Alignment Tool for easy alignment in editor
      (`/Game/FPSK/Blueprint/BP_MacroLibrary.AlignTool` (`self.AlignToReference`) (`self.Alignment`)))))