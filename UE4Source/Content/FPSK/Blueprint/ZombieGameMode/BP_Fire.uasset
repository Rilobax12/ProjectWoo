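; BP_Fire is a fire hazard actor that periodically damages every actor overlapping its box.
; The construction script sizes the box, particle spawn radius, light and sound attenuation from FireRadius, sets the particle spawn rate and starts the loop sound at a random offset.
; From BeginPlay, Hurt applies FireDamage, waits HurtRate, then calls itself again.
; A light flicker timeline exists but is never triggered.
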(event `Hurt`
  ;[0 0 0] Hurt overlapping actors
  (for _array_element (`PrimitiveComponent.GetOverlappingActors` (`self.Box`) null)
    (`GameplayStatics.ApplyDamage` _array_element (`self.FireDamage`) null self))
  (`KismetSystemLibrary.Delay` (`self.HurtRate`))
  (`self.Hurt`))

(event `self.ReceiveBeginPlay`
  ;[0 0 0] Hurt On Begin Play
  (`self.Hurt`))

(fn `UserConstructionScript`
  (bind _fireradius (`self.FireRadius`))
  (bind _pointlight (`self.PointLight`))
  ;[0 0 0] Fire construction
  ;;[1 1 1] Set particle/box extent/sound and light based on radius
  (`ParticleSystemComponent.SetFloatParameter` (`self.ParticleSystem`) "SpawnRadius" (`self.FireRadius`))
  (`BoxComponent.SetBoxExtent` (`self.Box`) (`KismetMathLibrary.MakeVector` _fireradius _fireradius 32.0) true)
  (`ParticleSystemComponent.SetFloatParameter` (`self.ParticleSystem`) "SpawnRate" (`self.FireSpawnRate`))
  (`PointLightComponent.SetAttenuationRadius` (`self.PointLight`) (* (`self.FireRadius`) 5.0))
  (`AudioComponent.AdjustAttenuation` (`self.WAV_FireLoop`) (make `SoundAttenuationSettings` :`FalloffDistance` (* (`self.FireRadius`) 10.0)))
  ;;[1 1 1] Play fire sound at random time
  (`AudioComponent.Play` (`self.WAV_FireLoop`) (`KismetMathLibrary.RandomFloatInRange` 0.0 1.0))
  ;;[1 1 1] Set default light variables
  (set `self.DefaultLightIntensity` (`LightComponentBase.Intensity` _pointlight))
  (set `self.DefaultLightLocation` (`SceneComponent.K2_GetComponentLocation` _pointlight)))