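; BP_ArmCamoChanger is an actor that changes a player's arm camo and hand skin when a FirstPersonCharacter enters its overlap sphere.
; An obstruction check gates the change, which applies the actor's clothes and hand materials by slot name to both character arm meshes and plays a whip sound.
; The construction script applies those materials, plus a head material, to the actor's own mesh, previewing the look it gives.
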(event `self.Sphere.OnComponentBeginOverlap`
  (params (OverlappedComponent :type "PrimitiveComponent Object Reference") (OtherActor :type "Actor Object Reference") (OtherComp :type "PrimitiveComponent Object Reference") (OtherBodyIndex :type Integer) (bFromSweep :type Boolean) (SweepResult :type "HitResult Structure (by ref)"))
  ;[0 0 0] Change camo logic
  ;;[1 1 1] If overlapping actor is a FirstPersonCharacter
  (bind _asfirst_person_character (cast `/Game/FPSK/FirstPersonAssets/FirstPersonBP/Blueprints/FirstPersonCharacter` OtherActor))
  ;;[1 1 1] Check if there is an obstruction between you and this actor
  (`/Game/FPSK/Blueprint/BP_MacroLibrary.ObstructionCheck` self _asfirst_person_character
    (:`No Obstruction`
      (bind _arms (`/Game/FPSK/FirstPersonAssets/FirstPersonBP/Blueprints/FirstPersonCharacter.Arms` _asfirst_person_character))
      ;;[1 1 1] Change arm material for player
      (`PrimitiveComponent.SetMaterialByName` _arms "Clothes" (`self.ClothesMaterial`))
      (`PrimitiveComponent.SetMaterialByName` (`/Game/FPSK/FirstPersonAssets/FirstPersonBP/Blueprints/FirstPersonCharacter.FirstPersonMesh` _asfirst_person_character) "Clothes" (`self.ClothesMaterial`))
      ;;[1 1 1] Set Hand material
      (`PrimitiveComponent.SetMaterialByName` _arms "Hands" (`self.HandSkinMaterial`))
      (`PrimitiveComponent.SetMaterialByName` (`/Game/FPSK/FirstPersonAssets/FirstPersonBP/Blueprints/FirstPersonCharacter.FirstPersonMesh` _asfirst_person_character) "Hands" (`self.HandSkinMaterial`))
      ;;[1 1 1] Play sound
      (`GameplayStatics.PlaySoundAtLocation` "/Game/FPSK/Sounds/WAV_Whip.WAV_Whip" (`self.K2_GetActorLocation`) (struct) 1.0 1.0 0.0 "/Game/FPSK/Sounds/Audio/Attenuation_CloseBy.Attenuation_CloseBy"))))

(fn `UserConstructionScript`
  ;[0 0 0] Set Arm material
  (`PrimitiveComponent.SetMaterialByName` (`self.Mesh`) "Clothes" (`self.ClothesMaterial`))
  ;[0 0 0] Set Hand material
  (`PrimitiveComponent.SetMaterialByName` (`self.Mesh`) "Hands" (`self.HandSkinMaterial`))
  ;[0 0 0] Set Head material
  (`PrimitiveComponent.SetMaterialByName` (`self.Mesh`) "Head" (`self.HeadSkinMaterial`)))