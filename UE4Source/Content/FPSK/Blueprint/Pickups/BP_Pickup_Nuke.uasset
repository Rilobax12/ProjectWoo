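; Nuke pickup for a zombie shooter that blows up all default zombies in the level when its effect triggers.
; It gives each zombie the character reference and sets a huge, strong ragdoll impulse centered on the pickup's location before calling Nuked on it.
; It then runs PickupEvent and shows a "Kaboom!" subtitle on the character's HUD.
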(event `self.PickupEffect`
  ;[0 0 0] Nuke Event
  ;;[1 1 1] For all zombies in level
  (bind _outactors (`GameplayStatics.GetAllActorsOfClass` "/Game/FPSK/Blueprint/Targets/BP_Target_DefaultZombie.BP_Target_DefaultZombie_C"))
  (for _array_element _outactors
    (set `/Game/FPSK/Blueprint/Targets/BP_Target.CharacterReference` (`self.CharacterReference`) _array_element)
    ;;[1 1 1] Set ragdoll physics
    (set `/Game/FPSK/Blueprint/Targets/BP_Target.HitLocation` (`self.K2_GetActorLocation`) _array_element)
    (set `/Game/FPSK/Blueprint/Targets/BP_Target.RagdollPhysicsRadius` 100000.0 _array_element)
    (set `/Game/FPSK/Blueprint/Targets/BP_Target.RagdollPhysicsStrength` 2500.0 _array_element)
    ;;[1 1 1] Nuke Target
    (`/Game/FPSK/Blueprint/Targets/BP_Target.Nuked` _array_element))
  (`self.PickupEvent`)
  ;;[1 1 1] Play subtitle
  (`/Game/FPSK/Blueprint/Widget/BP_MainHUD.PlaySubtitle` (`/Game/FPSK/FirstPersonAssets/FirstPersonBP/Blueprints/FirstPersonCharacter.MainHUD` (`self.CharacterReference`)) "Kaboom!" 2.0))

(fn `UserConstructionScript`
  (`parent.UserConstructionScript`))