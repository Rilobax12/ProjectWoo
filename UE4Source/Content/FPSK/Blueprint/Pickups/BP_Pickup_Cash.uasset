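; BP_Pickup_Cash is a pickup that gives the player money.
; Its PickupEffect event adds its Cash value to the Cash total stored on the character's MainHUD, then calls PickupEvent.
; It then plays the HUD's add/deduct animation with a "+$" amount label.
; The construction script only runs the parent's, so the rest of the pickup behavior is inherited.
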(event `self.PickupEffect`
  (bind _cash (`self.Cash`))
  (bind _mainhud (`/Game/FPSK/FirstPersonAssets/FirstPersonBP/Blueprints/FirstPersonCharacter.MainHUD` (`self.CharacterReference`)))
  ;[0 0 0] Add money
  ;;[1 1 1] Add cash for player
  (set `/Game/FPSK/Blueprint/Widget/BP_MainHUD.Cash` (+ (`/Game/FPSK/Blueprint/Widget/BP_MainHUD.Cash` _mainhud) _cash) _mainhud)
  (`self.PickupEvent`)
  (`/Game/FPSK/Blueprint/Widget/BP_MainHUD.PlayAddDeductAnimation` _mainhud (`KismetSystemLibrary.MakeLiteralText` (`KismetTextLibrary.Conv_StringToText` (`KismetStringLibrary.Concat_StrStr` "+$" (`KismetStringLibrary.Conv_IntToString` _cash)))) false))

(fn `UserConstructionScript`
  (`parent.UserConstructionScript`))