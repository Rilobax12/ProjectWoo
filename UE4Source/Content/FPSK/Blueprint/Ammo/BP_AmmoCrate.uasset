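; BP_AmmoCrate is an ammo crate actor that can rain gun pickups from above.
; RainGuns, gated by DropRandomWeapons, loops through a DoN and short delay to spawn a limited batch of randomly placed, rotated BP_GunPickups, calling attachment construction and timed self-destruction.
; Sphere end overlap clears the character's InteractReference; begin overlap is empty, leaving the logic that sets it disconnected.
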(event `self.Sphere.OnComponentBeginOverlap`
  (params (OverlappedComponent :type "PrimitiveComponent Object Reference") (OtherActor :type "Actor Object Reference") (OtherComp :type "PrimitiveComponent Object Reference") (OtherBodyIndex :type Integer) (bFromSweep :type Boolean) (SweepResult :type "HitResult Structure (by ref)"))
  ;[0 0 0] Overlap and End overlap events
)

(event `self.Sphere.OnComponentEndOverlap`
  (params (OverlappedComponent :type "PrimitiveComponent Object Reference") (OtherActor :type "Actor Object Reference") (OtherComp :type "PrimitiveComponent Object Reference") (OtherBodyIndex :type Integer))
  ;[0 0 0] Overlap and End overlap events
  ;;[1 1 1] Set Interact reference to none
  (bind _asfirst_person_character (cast `/Game/FPSK/FirstPersonAssets/FirstPersonBP/Blueprints/FirstPersonCharacter` OtherActor))
  (set `/Game/FPSK/FirstPersonAssets/FirstPersonBP/Blueprints/FirstPersonCharacter.InteractReference` null _asfirst_person_character))

(event `RainGuns`
  ;[0 0 0] Rain guns event
  (if (`self.DropRandomWeapons?`)
    (`|ExecutionSequence`
      (:`then_0`
        (goto _label :!via `Reset`))
      (:`then_1`
        (`/Engine/EditorBlueprintResources/StandardMacros.Do N` 20 :!label _label ; Amount of guns to spawn
          (:`Exit`
            (`|SpawnActorFromClass` "/Game/FPSK/Blueprint/BP_GunPickup.BP_GunPickup_C" (`KismetMathLibrary.MakeTransform` (+ (`self.K2_GetActorLocation`) (`KismetMathLibrary.MakeVector` (`KismetMathLibrary.RandomFloatInRange` -250.0 250.0) (`KismetMathLibrary.RandomFloatInRange` -250.0 250.0) 500.0)) (`KismetMathLibrary.RandomRotator` false)) "Undefined" "OverrideRootScale" null (struct) true false false null)
            (`/Game/FPSK/Blueprint/BP_GunPickup.Gun/AttachmentConstruction` (`self.Gun Reference`))
            ;;[1 1 1] Set gun lifetime
            (`/Game/FPSK/Blueprint/BP_GunPickup.DestroySelfAfterDelay` (`self.Gun Reference`) 20.0)
            ;;[1 1 1] Loop
            (`KismetSystemLibrary.Delay` 0.05)
            (goto _label)))))))

(fn `UserConstructionScript`)