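; Shootable target character serving as a flip-down course target, hostage or player-chasing zombie, depending on its flags.
; Point damage resolves headshots by bone or hitbox overlap, updates shooter HUD score and course stats, then ragdolls skeletal meshes or flips revivable static targets via timeline.
; Zombies AIMoveTo the nearest living player, turn on Tick for delayed, obstruction-checked bites, stun when hit, and on death notify the game mode and randomly drop pickups.
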(event `self.ReceiveTick`
  (params (DeltaSeconds :type "Float (single-precision)"))
  ;[0 0 0] Tick events
  (`self.LookAtTick`))

(event `DownTarget`
  (bind (_direction _rotation_alpha) (`Timeline|FlipTargetTimeline` :!label _label)
    (:`Update`
      (`SceneComponent.K2_SetRelativeRotation` (`self.Target`) (`KismetMathLibrary.RLerp` (struct :`Yaw` -90.0) (struct :`Yaw` -90.0 :`Roll` -90.0) _rotation_alpha) true false))))

(event `UpTarget`
  (goto _label :!via `Reverse`))

(event `Revive`
  (`PrimitiveComponent.SetCollisionEnabled` (`self.CapsuleComponent`) "QueryAndPhysics")
  (set `self.Health` (`self.MaxHealth`))
  (if (`self.Dead`)
    (`GameplayStatics.PlaySoundAtLocation` "/Game/FPSK/Sounds/WAV_WoodSwitch.WAV_WoodSwitch" (`self.K2_GetActorLocation`) (struct) 1.0 (`KismetMathLibrary.RandomFloatInRange` 1.0 1.5)))
  (set `self.Dead` false)
  (`self.UpTarget`))

(event `self.ReceivePointDamage`
  (params (Damage :type "Float (single-precision)") (DamageType :type "DamageType Object Reference") (HitLocation :type "Vector Structure") (HitNormal :type "Vector Structure") (HitComponent :type "PrimitiveComponent Object Reference") (BoneName :type Name) (ShotFromDirection :type "Vector Structure") (InstigatedBy :type "Controller Object Reference") (DamageCauser :type "Actor Object Reference") (HitInfo :type "HitResult Structure (by ref)"))
  (bind _coursevolume (`self.CourseVolume`))
  (bind _coursevolume_2 (`self.CourseVolume`))
  (bind _coursevolume_3 (`self.CourseVolume`))
  (bind _charactermovement (`self.CharacterMovement`))
  (bind _zombieanimation_bp (`self.ZombieAnimation_BP`))
  (bind _charactermovement_2 (`self.CharacterMovement`))
  (bind _coursevolume_4 (`self.CourseVolume`))
  (bind _returnvalue (- (`self.Health`) (`self.Damage`)))
  (bind _mainhud (`/Game/FPSK/FirstPersonAssets/FirstPersonBP/Blueprints/FirstPersonCharacter.MainHUD` (`self.CharacterReference`)))
  (if (not (`self.Dead`))
    (set `self.HitBone` BoneName)
    (set `self.RootDamage` Damage)
    (bind _output_get (set `self.HitLocation` HitLocation))
    (`SceneComponent.K2_SetWorldLocation` (`self.HitDetectionSphere`) _output_get false false)
    (bind _asfirst_person_character (cast `/Game/FPSK/FirstPersonAssets/FirstPersonBP/Blueprints/FirstPersonCharacter` DamageCauser))
    (set `self.CharacterReference` _asfirst_person_character)
    (set `self.CritShot` false)
    (`/Engine/EditorBlueprintResources/StandardMacros.IsValid` (`self.CharacterReference`)
      (:`Is Valid`
        (if (`/Game/FPSK/FirstPersonAssets/FirstPersonBP/Blueprints/FirstPersonCharacter.InstakillActive` (`self.CharacterReference`))
          (set `self.RootDamage` (`self.MaxHealth`)))
        (`|ExecutionSequence`
          (:`then_0`
            (`/Engine/EditorBlueprintResources/StandardMacros.IsValid` (`SkinnedMeshComponent.SkeletalMesh` (`self.Mesh`))
              (:`Is Valid`
                (if (== (`self.HitBone`) "Head")
                  (set `self.CritShot` true)))
              (:`Is Not Valid`
                (if (`PrimitiveComponent.IsOverlappingComponent` (`self.HitDetectionSphere`) (`self.HeadHitbox`))
                  (set `self.CritShot` true)))))
          (:`then_1`
            (if (`self.CritShot`)
              (set `self.Damage` (* (`self.RootDamage`) (`self.HeadshotDamageMultiplier`)))))
          (:`then_2`
            (set `self.Previous Health` (`self.Health`))
            (if (`self.CritShot`)
              (`/Game/FPSK/Blueprint/Widget/BP_MainHUD.HitmarkerCrit` _mainhud)
              (else
                (set `self.Damage` (`self.RootDamage`))
                (`/Game/FPSK/Blueprint/Widget/BP_MainHUD.Hitmarker` _mainhud)))
            (set `self.Health` (`KismetMathLibrary.SelectFloat` _returnvalue (`KismetMathLibrary.FClamp` _returnvalue 0.0 (`self.MaxHealth`)) (`self.Invincible`)))
            (if false
              (`KismetSystemLibrary.PrintString` (`KismetStringLibrary.Concat_StrStr` "Damage: " (`KismetStringLibrary.Conv_DoubleToString` (`self.Damage`))) true true (struct :`R` 1.0 :`G` 1.0 :`B` 1.0 :`A` 1.0)))
            (`/Engine/EditorBlueprintResources/StandardMacros.IsValid` _coursevolume
              (:`Is Valid`
                (if (`/Game/FPSK/Blueprint/CourseLogic/BP_CourseVolume.CourseRuntimeActive` _coursevolume)
                  (`/Engine/EditorBlueprintResources/StandardMacros.IncrementInt` (`/Game/FPSK/Blueprint/CourseLogic/BP_CourseVolume.HitCount` _coursevolume_4)
                    (:`  `
                      (if (`self.CritShot`)
                        (`/Engine/EditorBlueprintResources/StandardMacros.IncrementInt` (`/Game/FPSK/Blueprint/CourseLogic/BP_CourseVolume.CriticalHitCount` _coursevolume_4)
                          (:`  `
                            _)))))))
              (:`Is Not Valid`
                _))
            (if (`self.GivePointsOnHit`)
              (if (`self.IsHostage?`)
                (`self.DeductScore` (`self.ScoreOnHit`))
                (`/Engine/EditorBlueprintResources/StandardMacros.IsValid` _coursevolume_2
                  (:`Is Valid`
                    (if (`/Game/FPSK/Blueprint/CourseLogic/BP_CourseVolume.CourseRuntimeActive` _coursevolume_2)
                      (`GameplayStatics.PlaySound2D` "/Game/FPSK/Sounds/WAV_HostageShot.WAV_HostageShot")))
                  (:`Is Not Valid`
                    _))
                (else
                  (`/Engine/EditorBlueprintResources/StandardMacros.CompareFloat` (`self.Previous Health`) (`self.Health`)
                    (:`>`
                      (`self.AddScore` (* (`KismetMathLibrary.Round` (- (`self.Previous Health`) (`self.Health`))) (`self.ScoreOnHit`))))
                    (:`==`
                      _)
                    (:`<`
                      _)))))
            (`/Engine/EditorBlueprintResources/StandardMacros.CompareFloat` (`self.Health`)
              (:`>`
                (if (`self.FollowingZombie`)
                  (set `self.HitStunned` true)
                  (`|ExecutionSequence`
                    (:`then_0`
                      (`/Engine/EditorBlueprintResources/StandardMacros.IsValid` (`self.ZombieSnarl`)
                        (:`Is Valid`
                          (`AudioComponent.Stop` (`self.ZombieSnarl`))
                          (`self.ResetZombieSoundDoOnce`))
                        (:`Is Not Valid`
                          _))
                      (`GameplayStatics.PlaySoundAtLocation` "/Game/FPSK/Sounds/WAV_ZombieHit.WAV_ZombieHit" (`self.K2_GetActorLocation`) (struct) 0.35 (`KismetMathLibrary.RandomFloatInRange` 0.5 1.0))
                      (if (not (`NavMovementComponent.IsFalling` (`self.CharacterMovement`)))
                        (`NavMovementComponent.StopActiveMovement` _charactermovement_2)
                        (`CharacterMovementComponent.DisableMovement` _charactermovement_2)
                        (`KismetSystemLibrary.RetriggerableDelay` (`self.HitStunDuration`))
                        (set `self.HitStunned` false)
                        (`CharacterMovementComponent.SetMovementMode` (`self.CharacterMovement`) "MOVE_Walking" 0)
                        (`self.RefollowCharacter`)))
                    (:`then_1`
                      (`/Engine/EditorBlueprintResources/StandardMacros.IsValid` _zombieanimation_bp
                        (:`Is Valid`
                          (if (not (`AnimInstance.IsPlayingSlotAnimation` _zombieanimation_bp "/Game/FPSK/Animations/Zombie/A_Zombie_Bite.A_Zombie_Bite" "UpperBody"))
                            (`AnimInstance.PlaySlotAnimation` (`self.ZombieAnimation_BP`) "/Game/FPSK/Animations/Zombie/A_Zombie_Hit.A_Zombie_Hit" "UpperBody" 0.1 0.25 1.0 1))))))))
              (:`==`
                (if (not (`self.Invincible`)) :!label _label_2
                  (`/Engine/EditorBlueprintResources/StandardMacros.IsValid` (`SkinnedMeshComponent.SkeletalMesh` (`self.Mesh`)) :!label _label_3
                    (:`Is Valid`
                      (`PrimitiveComponent.SetSimulatePhysics` (`self.Mesh`) true)
                      (`PrimitiveComponent.AddRadialImpulse` (`self.Mesh`) (`self.HitLocation`) (`self.RagdollPhysicsRadius`) (`self.RagdollPhysicsStrength`) "RIF_Constant" true))
                    (:`Is Not Valid`
                      (`self.DownTarget`)
                      (`GameplayStatics.PlaySoundAtLocation` "/Game/FPSK/Sounds/WAV_WoodSwitch.WAV_WoodSwitch" (`self.K2_GetActorLocation`) (struct) 1.0 (`KismetMathLibrary.RandomFloatInRange` 1.0 1.5) 0.0 "/Game/FPSK/Sounds/Audio/Attenuation_FarRange.Attenuation_FarRange")))
                  (set `self.Dead` true)
                  (`MovementComponent.StopMovementImmediately` (`self.CharacterMovement`))
                  (`PrimitiveComponent.SetCollisionEnabled` (`self.CapsuleComponent`) "NoCollision")
                  (`/Engine/EditorBlueprintResources/StandardMacros.IsValid` (`self.CourseVolume`)
                    (:`Is Valid`
                      (if (`/Game/FPSK/Blueprint/CourseLogic/BP_CourseVolume.CourseRuntimeActive` (`self.CourseVolume`))
                        (if (`self.IsHostage?`)
                          (if (not (`self.GivePointsOnHit`))
                            (`GameplayStatics.PlaySound2D` "/Game/FPSK/Sounds/WAV_HostageShot.WAV_HostageShot"))
                          (else
                            (`GameplayStatics.PlaySound2D` "/Game/FPSK/Sounds/WAV_EnemyKill.WAV_EnemyKill")))))
                    (:`Is Not Valid`
                      _))
                  (if (`self.CurrentlyPartOfCourse`)
                    (`/Engine/EditorBlueprintResources/StandardMacros.IsValid` _coursevolume_3
                      (:`Is Valid`
                        (`/Game/FPSK/Blueprint/CourseLogic/BP_CourseVolume.KillCheck` _coursevolume_3))
                      (:`Is Not Valid`
                        _)))
                  (if (`self.FollowingZombie`)
                    (`|ExecutionSequence`
                      (:`then_0`
                        (bind _asbp_zombie_game_mode (cast `/Game/FPSK/Blueprint/ZombieGameMode/BP_ZombieGameMode` (`GameplayStatics.GetGameMode`)))
                        (bind _result (`/Engine/EditorBlueprintResources/StandardMacros.IncrementInt` (`/Game/FPSK/Blueprint/ZombieGameMode/BP_ZombieGameMode.KillCount` _asbp_zombie_game_mode))
                          (:`  `
                            (set `/Game/FPSK/Blueprint/ZombieGameMode/BP_ZombieGameMode.KillCount` _result _asbp_zombie_game_mode)
                            (`/Game/FPSK/Blueprint/ZombieGameMode/BP_ZombieGameMode.KillCheck` _asbp_zombie_game_mode))))
                      (:`then_1`
                        (`NavMovementComponent.StopActiveMovement` _charactermovement)
                        (`CharacterMovementComponent.DisableMovement` _charactermovement)
                        (`/Engine/EditorBlueprintResources/StandardMacros.IsValid` (`self.ZombieSnarl`)
                          (:`Is Valid`
                            (`AudioComponent.Stop` (`self.ZombieSnarl`)))
                          (:`Is Not Valid`
                            _))
                        (`GameplayStatics.PlaySoundAtLocation` "/Game/FPSK/Sounds/WAV_ZombieDie.WAV_ZombieDie" (`self.K2_GetActorLocation`) (struct) 0.35 (`KismetMathLibrary.RandomFloatInRange` 0.5 1.5))
                        (`KismetSystemLibrary.Delay` 5.0)
                        (for _array_element (`self.GetAttachedActors`)
                          (`self.K2_DestroyActor` _array_element))
                        (`self.K2_DestroyActor`))
                      (:`then_2`
                        (`self.DropMacro` "/Game/FPSK/Blueprint/Pickups/BP_Pickup_Cash.BP_Pickup_Cash_C" 8.0 30.0)
                        (`self.DropMacro` "/Game/FPSK/Blueprint/Pickups/BP_Pickup_Health.BP_Pickup_Health_C" 8.0 30.0)
                        (`self.DropMacro` "/Game/FPSK/Blueprint/Pickups/BP_Pickup_AmmoRefill.BP_Pickup_AmmoRefill_C" 8.0 30.0)
                        (`self.DropMacro` "/Game/FPSK/Blueprint/Pickups/BP_Pickup_Instakill.BP_Pickup_Instakill_C" 4.0 30.0)
                        (`self.DropMacro` "/Game/FPSK/Blueprint/Pickups/BP_Pickup_Nuke.BP_Pickup_Nuke_C" 1.0 30.0))
                      (:`then_3`
                        (if (and (`self.GivePointsOnKill`) (not (`self.IsNuked`))) :!label _label_4
                          (if (not (`self.IsHostage?`))
                            (if (`self.GivePointsOnKill`)
                              (`self.AddScore` (`KismetMathLibrary.SelectInt` (`KismetMathLibrary.SelectInt` (`KismetMathLibrary.FFloor` (* (`self.ScoreOnKill`) (`self.HeadshotScoreMultiplier`))) (`self.ScoreOnKill`) (`self.CritShot`)) (`self.ScoreOnKill`) (`self.CriticalHitScoreBonus`)) 1))
                            (elif (`self.GivePointsOnKill`)
                              (`self.DeductScore` (`self.ScoreOnKill`)))))))
                    (else
                      (goto _label_4)))))
              (:`<`
                (goto _label_2)))))))))

(event `Nuked`
  (if (not (`self.Dead`))
    (set `self.IsNuked` true) ; Set Nuked state, does not add points if nuked
    (`/Engine/EditorBlueprintResources/StandardMacros.DoOnce` false
      (:`Completed`
        (goto _label_3)))))

(event `self.ReceivePossessed`
  (params (NewController :type "Controller Object Reference"))
  ;[0 0 0] Begin Play events
  (`KismetSystemLibrary.Delay` 0.2)
  (`self.TargetCharacter`))

(event `LookAtTick`
  (bind _followtarget (`self.Followtarget`))
  (bind _zombieanimation_bp (`self.ZombieAnimation_BP`))
  (bind _returnvalue (`KismetMathLibrary.FindLookAtRotation` (`self.K2_GetActorLocation`) (`self.K2_GetActorLocation` (`self.Followtarget`))))
  (`/Engine/EditorBlueprintResources/StandardMacros.IsValid` (`self.Followtarget`)
    (:`Is Valid`
      (if (and (`self.FocusedPlayer`) (not (`self.HitStunned`)) (not (`self.Dead`)))
        (`/Engine/EditorBlueprintResources/StandardMacros.IsValid` _followtarget
          (:`Is Valid`
            (if (not (`/Game/FPSK/FirstPersonAssets/FirstPersonBP/Blueprints/FirstPersonCharacter.IsDead` _followtarget))
              (set `self.PlayerFocusRotation` (`KismetMathLibrary.MakeRotator` 0.0 0.0 (.yaw _returnvalue)))
              (`self.K2_SetActorRotation` (`KismetMathLibrary.RInterpTo` (`self.K2_GetActorRotation`) (`KismetMathLibrary.MakeRotator` (.roll (`self.K2_GetActorRotation`)) (.pitch (`self.K2_GetActorRotation`)) (.yaw _returnvalue)) (`GameplayStatics.GetWorldDeltaSeconds`) (`self.FacePlayerRotationSpeed`)))
              (if (== (`KismetMathLibrary.MakeRotator` 0.0 0.0 (.yaw (`self.K2_GetActorRotation`))) (`self.PlayerFocusRotation`) :`ErrorTolerance` (`self.AcceptableBiteAngle`))
                (`/Engine/EditorBlueprintResources/StandardMacros.CompareFloat` (`self.GetDistanceTo` (`self.Followtarget`)) (+ (`self.AttackRadius`) 100.0)
                  (:`>`
                    (`self.RefollowCharacter` :!label _label_5))
                  (:`==`
                    (goto _label_5))
                  (:`<`
                    (`KismetSystemLibrary.Delay` (`self.BiteDelay`))
                    (`/Engine/EditorBlueprintResources/StandardMacros.IsValid` (`self.Followtarget`)
                      (:`Is Valid`
                        (if (and (`self.FocusedPlayer`) (not (`self.Dead`)) (not (`/Game/FPSK/FirstPersonAssets/FirstPersonBP/Blueprints/FirstPersonCharacter.IsDead` (`self.Followtarget`))))
                          (`/Game/FPSK/Blueprint/BP_MacroLibrary.ObstructionCheck` self (`self.Followtarget`)
                            (:`No Obstruction`
                              (`GameplayStatics.ApplyDamage` (`self.Followtarget`) (`self.ZombieBiteDamage`))
                              (`GameplayStatics.PlaySoundAtLocation` "/Game/FPSK/Sounds/WAV_ZombieBite.WAV_ZombieBite" (`self.K2_GetActorLocation`))
                              (`/Engine/EditorBlueprintResources/StandardMacros.IsValid` _zombieanimation_bp
                                (:`Is Valid`
                                  (`AnimInstance.PlaySlotAnimation` _zombieanimation_bp "/Game/FPSK/Animations/Zombie/A_Zombie_Bite.A_Zombie_Bite" "UpperBody" 0.1 0.25 1.0 1))))
                            (:`Blocked`
                              (`self.RefollowCharacter` :!label _label_6)))
                          (else
                            (goto _label_6))))
                      (:`Is Not Valid`
                        (goto _label_6)))))))))))
    (:`Is Not Valid`
      (`self.RefollowCharacter`))))

(event `TargetCharacter`
  (bind _target (`self.Target`))
  (if (and (not (`self.Dead`)) (`self.FollowingZombie`)) :!label _label_7
    (`|ExecutionSequence`
      (:`then_0`
        (`/Engine/EditorBlueprintResources/StandardMacros.DoOnce` false :!label _label_8
          (:`Completed`
            (bind _returnvalue (`GameplayStatics.SpawnSoundAttached` "/Game/FPSK/Sounds/WAV_ZombieSnarl.WAV_ZombieSnarl" _target "None" (`SceneComponent.K2_GetComponentLocation` _target) (struct) "KeepWorldPosition" true 1.0 1.0 (`KismetMathLibrary.RandomFloatInRange` 0.0 55.0) "/Game/FPSK/Sounds/Audio/Attenuation_FarRange.Attenuation_FarRange"))
            (set `self.ZombieSnarl` _returnvalue))))
      (:`then_1`
        (`self.GetClosestCharacter`)
        (`AITask_MoveTo.AIMoveTo` (`AIBlueprintHelperLibrary.GetAIController` self) (0.0 0.0 0.0) (`self.Followtarget`) (`self.AttackRadius`) "Default" "Default" true false
          (:`OnRequestFailed`
            (set `self.Followtarget` null))
          (:`OnMoveFinished`
            (set `self.FocusedPlayer` true)))))))

(event `ResetZombieSoundDoOnce`
  (goto _label_8 :!via `Reset`))

(event `self.OnLanded`
  (params (Hit :type "HitResult Structure (by ref)"))
  (goto _label_7))

(fn `AddScore`
  (params (`Added Score` :type Integer) (`Added Multiplier` :type Integer) (`Reset Multiplier?` :type Boolean))
  (bind _mainhud (`/Game/FPSK/FirstPersonAssets/FirstPersonBP/Blueprints/FirstPersonCharacter.MainHUD` (`self.CharacterReference`)))
  (`self.CourseTargetCheck`
    (:`Output`
      (set `/Game/FPSK/Blueprint/Widget/BP_MainHUD.ScoreDisplay` (+ (`/Game/FPSK/Blueprint/Widget/BP_MainHUD.ScoreDisplay` _mainhud) `Added Score`) _mainhud)
      (set `/Game/FPSK/Blueprint/Widget/BP_MainHUD.Multiplier` (`KismetMathLibrary.SelectInt` 0 (+ (`/Game/FPSK/Blueprint/Widget/BP_MainHUD.Multiplier` _mainhud) `Added Multiplier`) `Reset Multiplier?`) _mainhud)
      (`/Game/FPSK/Blueprint/Widget/BP_MainHUD.ScorePopinAnimation` _mainhud))))

(fn `DeductScore`
  (params (`Deducted Score` :type Integer))
  (bind _mainhud (`/Game/FPSK/FirstPersonAssets/FirstPersonBP/Blueprints/FirstPersonCharacter.MainHUD` (`self.CharacterReference`)))
  (`self.CourseTargetCheck`
    (:`Output`
      (set `/Game/FPSK/Blueprint/Widget/BP_MainHUD.Multiplier` 0 _mainhud)
      (set `/Game/FPSK/Blueprint/Widget/BP_MainHUD.Score` (- (`/Game/FPSK/Blueprint/Widget/BP_MainHUD.Score` _mainhud) `Deducted Score`) _mainhud)
      (`/Game/FPSK/Blueprint/Widget/BP_MainHUD.ScoreDeductEvent` _mainhud (`KismetTextLibrary.Conv_StringToText` (`KismetStringLibrary.Concat_StrStr` "-" (`KismetStringLibrary.Conv_IntToString` `Deducted Score`)))))))

(fn `GetClosestCharacter`
  (bind _closestplayerreference (`self.ClosestPlayerReference`))
  ;[1 1 1] Clear live players array
  (`KismetArrayLibrary.Array_Clear` (`self.LivePlayers`))
  ;[1 1 1] Add all live players to array
  (bind _outactors (`GameplayStatics.GetAllActorsOfClass` "/Game/FPSK/FirstPersonAssets/FirstPersonBP/Blueprints/FirstPersonCharacter.FirstPersonCharacter_C"))
  (for _array_element _outactors
    (if (not (`/Game/FPSK/FirstPersonAssets/FirstPersonBP/Blueprints/FirstPersonCharacter.IsDead` _array_element))
      (`KismetArrayLibrary.Array_Add` (`self.LivePlayers`) _array_element)))
  ;[1 1 1] If there is any live players found
  (if (> (`KismetArrayLibrary.Array_Length` (`self.LivePlayers`)) 0)
    ;[1 1 1] Set first closest player reference
    (bind _output_get (set `self.ClosestPlayerReference` (`|GetArrayItem` (`self.LivePlayers`))))
    (`/Engine/EditorBlueprintResources/StandardMacros.IsValid` _output_get
      (:`Is Valid`
        (`|ExecutionSequence`
          (:`then_0`
            ;[1 1 1] Must set first distance check to any player for compare loop
            (`/Engine/EditorBlueprintResources/StandardMacros.IsValid` _closestplayerreference
              (:`Is Valid`
                (set `self.ClosestPlayerDistance` (`self.GetDistanceTo` _closestplayerreference)))))
          (:`then_1`
            ;[1 1 1] For all live targets
            (for _array_element_2 (`self.LivePlayers`)
              ;[1 1 1] Check if still alive for good measure
              (bind _output_get_2 (set `self.ClosestPlayerReference` _array_element_2))
              (if (not (`/Game/FPSK/FirstPersonAssets/FirstPersonBP/Blueprints/FirstPersonCharacter.IsDead` _output_get_2))
                ;[1 1 1] Check if distance is closer than any previous checks
                (bind _output_get_3 (set `self.CurrentPlayerDistance` (`self.GetDistanceTo` (`self.ClosestPlayerReference`))))
                (`/Engine/EditorBlueprintResources/StandardMacros.CompareFloat` _output_get_3 (`self.ClosestPlayerDistance`)
                  (:`==`
                    _)
                  (:`<`
                    _))
                ;[1 1 1] Set Closest player and set Closest Player Distance if closer to target
                (set `self.Followtarget` (`self.ClosestPlayerReference`))
                (set `self.ClosestPlayerDistance` (`self.CurrentPlayerDistance`))))))))
    (else
      ;[1 1 1] Set Follow target to none if there are no live targets found
      (set `self.Followtarget` null))))

(fn `RefollowCharacter`
  (set `self.FocusedPlayer` false)
  (set `self.Followtarget` null)
  (`self.TargetCharacter`))

(fn `UserConstructionScript`
  (bind _returnvalue (`self.K2_GetActorLocation`))
  ;[0 0 0] Target construction
  (`|ExecutionSequence`
    (:`then_0`
      ;;[1 1 1] Set health to max health
      (set `self.Health` (`self.MaxHealth`))
      ;;[1 1 1] Set mesh and silhouette
      (if (`self.UseSillhouette`)
        (`StaticMeshComponent.SetStaticMesh` (`self.Target`) (`self.TargetMesh`))
        (bind _returnvalue_2 (`PrimitiveComponent.CreateDynamicMaterialInstance` (`self.Target`) 0 null))
        (`MaterialInstanceDynamic.SetVectorParameterValue` _returnvalue_2 "Color" (`self.SilhouetteColor`))
        (`MaterialInstanceDynamic.SetTextureParameterValue` _returnvalue_2 "Outline" (`self.SilhouetteTexture`)))
      ;;[1 1 1] Set movement speed for Zombie setting
      (set `CharacterMovementComponent.MaxWalkSpeed` (`self.MovementSpeed`) (`self.CharacterMovement`))
      ;[0 0 0] Align to floor if true
      (if (`self.AlignToGroundAngle`)
        ;;[1 1 1] Trace to the ground
        (bind _outhit (`KismetSystemLibrary.LineTraceSingle` :`Start` _returnvalue :`End` (+ _returnvalue (* (`KismetMathLibrary.GetUpVector` (`self.K2_GetActorRotation`)) -500.0)) :`TraceChannel` "TraceTypeQuery1" :`DrawDebugType` "ForDuration"))
        ;;[1 1 1] Set actor rotation based on ground angle + offset
        (`self.K2_SetActorRotation` (`KismetMathLibrary.NegateRotator` (`KismetMathLibrary.ComposeRotators` (`KismetMathLibrary.NegateRotator` (`KismetMathLibrary.MakeRotFromZ` (`.Normal` (`GameplayStatics.BreakHitResult` _outhit)))) (`self.NormalRotationOffset`))))))
    (:`then_1`
      ;;[1 1 1] Hide Target if there is a skeletal mesh
      (`/Engine/EditorBlueprintResources/StandardMacros.IsValid` (`SkinnedMeshComponent.SkeletalMesh` (`self.Mesh`))
        (:`Is Valid`
          (`SceneComponent.SetVisibility` (`self.Target`) false true)
          ;;[1 1 1] Turn off collision for target mesh
          (`PrimitiveComponent.SetCollisionEnabled` (`self.Target`) "NoCollision")
          ;;[1 1 1] If Zombie, set animation BP reference
          (if (`self.FollowingZombie`)
            _))))))