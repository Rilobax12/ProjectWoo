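; Box trigger that starts or finishes a shooting course on its referenced course volume when a FirstPersonCharacter overlaps it.
; Start triggers require an inactive course and character; end triggers require the initiator, an active course and all enemies dead, and each hides its sibling markers on firing.
; Resettable DoOnce nodes prevent repeats, and a gate ignores overlaps until just after BeginPlay.
; Construction styles end triggers as hidden FINISH markers and disables the volume's finish-on-all-dead option.
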(event `self.Box.OnComponentBeginOverlap`
  (params (OverlappedComponent :type "PrimitiveComponent Object Reference") (OtherActor :type "Actor Object Reference") (OtherComp :type "PrimitiveComponent Object Reference") (OtherBodyIndex :type Integer) (bFromSweep :type Boolean) (SweepResult :type "HitResult Structure (by ref)"))
  (bind _coursevolumereference (`self.CourseVolumeReference`))
  (bind _coursevolumereference_2 (`self.CourseVolumeReference`))
  (bind _courseinitiatorcharacter (`/Game/FPSK/Blueprint/CourseLogic/BP_CourseVolume.CourseInitiatorCharacter` _coursevolumereference))
  ;[0 0 0] Communicate overlap event with course volume BP
  (`/Engine/EditorBlueprintResources/StandardMacros.Gate` true :!label _label
    (:`Exit`
      (bind _asfirst_person_character (cast `/Game/FPSK/FirstPersonAssets/FirstPersonBP/Blueprints/FirstPersonCharacter` OtherActor))
      ;;[1 1 1] Can only trigger event if not currently in course
      (bind _output_get (set `self.OverlappingCharacter` _asfirst_person_character))
      (if (not (`/Game/FPSK/FirstPersonAssets/FirstPersonBP/Blueprints/FirstPersonCharacter.CurrentlyInCourse` _output_get))
        (`/Engine/EditorBlueprintResources/StandardMacros.IsValid` (`self.CourseVolumeReference`) :!label _label_2
          (:`Is Valid`
            (if (`self.IsEndTrigger?`)
              ;;[1 1 1] Only finish course if currently active + overlapping character = course initiator + all anemies are dead
              (`/Engine/EditorBlueprintResources/StandardMacros.IsValid` _courseinitiatorcharacter
                (:`Is Valid`
                  (if (and (== _courseinitiatorcharacter (`self.OverlappingCharacter`)) (`/Game/FPSK/Blueprint/CourseLogic/BP_CourseVolume.CourseActive` _coursevolumereference) (== (`/Game/FPSK/Blueprint/CourseLogic/BP_CourseVolume.DeadEnemiesCount` _coursevolumereference_2) (`/Game/FPSK/Blueprint/CourseLogic/BP_CourseVolume.EnemyCount` _coursevolumereference_2)))
                    (`/Engine/EditorBlueprintResources/StandardMacros.DoOnce` false :!label _label_3
                      (:`Completed`
                        (`/Game/FPSK/Blueprint/CourseLogic/BP_CourseVolume.TriggerFinish` (`self.CourseVolumeReference`))
                        ;;[1 1 1] Hide all course end triggers
                        (for _array_element (`/Game/FPSK/Blueprint/CourseLogic/BP_CourseVolume.CourseEndTriggers` (`self.CourseVolumeReference`))
                          (`SceneComponent.SetHiddenInGame` (`/Game/FPSK/Blueprint/CourseLogic/BP_CourseTrigger.Marker` _array_element) true true)))))))
              (else
                ;;[1 1 1] Only activate if course currently not active
                (if (not (`/Game/FPSK/Blueprint/CourseLogic/BP_CourseVolume.CourseActive` (`self.CourseVolumeReference`)))
                  (`/Engine/EditorBlueprintResources/StandardMacros.DoOnce` false :!label _label_4
                    (:`Completed`
                      (`/Game/FPSK/Blueprint/CourseLogic/BP_CourseVolume.TriggerStart` (`self.CourseVolumeReference`) OtherActor)
                      ;;[1 1 1] Hide all course start triggers
                      (for _array_element_2 (`/Game/FPSK/Blueprint/CourseLogic/BP_CourseVolume.CourseStartTriggers` (`self.CourseVolumeReference`))
                        (`SceneComponent.SetHiddenInGame` (`/Game/FPSK/Blueprint/CourseLogic/BP_CourseTrigger.Marker` _array_element_2) true true)))))))))
        (else
          ;;[1 1 1] Check if end trigger
          (if (`self.IsEndTrigger?`)
            (goto _label_2)))))))

(event `ResetTriggerDoOnce`
  ;[0 0 0] Communicate overlap event with course volume BP
  (`|ExecutionSequence`
    (:`then_0`
      (goto _label_3 :!via `Reset`))
    (:`then_1`
      (goto _label_4 :!via `Reset`))))

(event `self.ReceiveBeginPlay`
  ;[0 0 0] Communicate overlap event with course volume BP
  (`KismetSystemLibrary.Delay` 0.0) ; Let construction scripts run before overlapping, this prevents errors if you begin play overlapping the trigger
  (goto _label :!via `Open`))

(fn `UpdateColor`
  (bind _textrendercolor (`TextRenderComponent.TextRenderColor` (`self.TextRender`)))
  (bind _returnvalue (`KismetMathLibrary.Conv_ColorToLinearColor` _textrendercolor))
  ;[0 0 0] Update Color
  ;;[1 1 1] Set emissive colors based on first text render color
  (bind _returnvalue_2 (`PrimitiveComponent.CreateDynamicMaterialInstance` (`self.Marker`) 1 null))
  (`MaterialInstanceDynamic.SetVectorParameterValue` _returnvalue_2 "Color" _returnvalue)
  (`TextRenderComponent.SetTextRenderColor` (`self.TextRenderMirror`) _textrendercolor)
  (`LightComponent.SetLightColor` (`self.PointLight`) _returnvalue true))

(fn `UserConstructionScript`
  ;[0 0 0] Trigger construction
  ;;[1 1 1] Set trigger box extent
  (`BoxComponent.SetBoxExtent` (`self.Box`) (`self.Trigger Box Extent`) true)
  (`self.UpdateColor`)
  (if (`self.IsEndTrigger?`)
    ;;[1 1 1] Set mesh settings for end trigger
    (`TextRenderComponent.K2_SetText` (`self.TextRender`) "FINISH")
    (`TextRenderComponent.K2_SetText` (`self.TextRenderMirror`) "FINISH")
    (`TextRenderComponent.SetTextRenderColor` (`self.TextRender`) (`self.FinishColor`))
    (`self.UpdateColor`)
    (`SceneComponent.SetHiddenInGame` (`self.Marker`) true true)
    ;;[1 1 1] Set use trigger end for course volume reference
    (`/Engine/EditorBlueprintResources/StandardMacros.IsValid` (`self.CourseVolumeReference`)
      (:`Is Valid`
        (set `/Game/FPSK/Blueprint/CourseLogic/BP_CourseVolume.FinishOnAllDeadTargets` false (`self.CourseVolumeReference`))))))