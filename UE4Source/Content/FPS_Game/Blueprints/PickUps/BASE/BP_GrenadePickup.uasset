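; BP_GrenadePickup is an interactable pickup that gives the player one grenade.
; On BeginPlay it casts player character 0 to BP_CharacterBase and caches the reference.
; The BPIInteraction event compares the player's current grenade count to the maximum, then either calls AddGrenades and destroys the pickup or prints a max-grenades message and leaves it in place.
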(event `self.ReceiveBeginPlay`
  (bind _asbp_character_base (cast `/Game/FPS_Game/Blueprints/BP_CharacterBase` (`GameplayStatics.GetPlayerCharacter` 0)))
  (set `self.PlayerCast` _asbp_character_base))

(event `/Game/FPS_Game/Blueprints/System/BPI_Interact.BPI_Interaction`
  (bind _playercast (`self.PlayerCast`))
  (`/Engine/EditorBlueprintResources/StandardMacros.CompareInt` (`/Game/FPS_Game/Blueprints/BP_CharacterBase.CurrentGrenades` _playercast) (`/Game/FPS_Game/Blueprints/BP_CharacterBase.MaxGrenades` _playercast)
    (:`>`
      (`KismetSystemLibrary.PrintString` "MAX  GRENADES" :!label _label))
    (:`==`
      (goto _label))
    (:`<`
      (`/Game/FPS_Game/Blueprints/BP_CharacterBase.AddGrenades` _playercast 1)
      (`KismetSystemLibrary.PrintString` "GRENADE  ADDED")
      (`self.K2_DestroyActor`))))

(fn `UserConstructionScript`)