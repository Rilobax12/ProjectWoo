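; Climbable ladder actor whose length follows the LadderHeight vector.
; The construction script stacks instanced mesh segments up to that height and resizes and offsets the overlap box to cover them.
; Entering the box switches a FirstPersonCharacter to Flying movement, sets its Climbing flag and calls Climb.
; Leaving restores Walking, clears the flag and calls Unclimb, leaving climb behavior to the character Blueprint.
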(event `self.Box.OnComponentBeginOverlap`
  (params (OverlappedComponent :type "PrimitiveComponent Object Reference") (OtherActor :type "Actor Object Reference") (OtherComp :type "PrimitiveComponent Object Reference") (OtherBodyIndex :type Integer) (bFromSweep :type Boolean) (SweepResult :type "HitResult Structure (by ref)"))
  (bind _characterreference (`self.CharacterReference`))
  ;[0 0 0] Climb events
  ;;[1 1 1] Cast to character and set to variable
  (bind _asfirst_person_character (cast `/Game/FPSK/FirstPersonAssets/FirstPersonBP/Blueprints/FirstPersonCharacter` OtherActor))
  (bind _output_get (set `self.CharacterReference` _asfirst_person_character))
  ;;[1 1 1] Set to flying movement mode
  (`CharacterMovementComponent.SetMovementMode` (`Character.CharacterMovement` _output_get) "MOVE_Flying" 0)
  ;;[1 1 1] Set climbing state and run climb event in character blueprint
  (set `/Game/FPSK/FirstPersonAssets/FirstPersonBP/Blueprints/FirstPersonCharacter.Climbing` true _characterreference)
  (`/Game/FPSK/FirstPersonAssets/FirstPersonBP/Blueprints/FirstPersonCharacter.Climb` _characterreference))

(event `self.Box.OnComponentEndOverlap`
  (params (OverlappedComponent :type "PrimitiveComponent Object Reference") (OtherActor :type "Actor Object Reference") (OtherComp :type "PrimitiveComponent Object Reference") (OtherBodyIndex :type Integer))
  (bind _characterreference (`self.CharacterReference`))
  ;[0 0 0] Unclimb events
  ;;[1 1 1] Cast to character and set to variable
  (bind _asfirst_person_character (cast `/Game/FPSK/FirstPersonAssets/FirstPersonBP/Blueprints/FirstPersonCharacter` OtherActor))
  (bind _output_get (set `self.CharacterReference` _asfirst_person_character))
  ;;[1 1 1] Set back to walking movement mode
  (`CharacterMovementComponent.SetMovementMode` (`Character.CharacterMovement` _output_get) "MOVE_Walking" 0)
  ;;[1 1 1] Set climbing state off and run unclimb event in character blueprint
  (set `/Game/FPSK/FirstPersonAssets/FirstPersonBP/Blueprints/FirstPersonCharacter.Climbing` false _characterreference)
  (`/Game/FPSK/FirstPersonAssets/FirstPersonBP/Blueprints/FirstPersonCharacter.Unclimb` _characterreference))

(fn `UserConstructionScript`
  (bind _returnvalue (* 25.0 (/ (.z (`self.LadderHeight`)) 50.0)))
  ;[0 0 0] Ladder construction
  ;;[1 1 1] Add instanced static mesh
  (bind _returnvalue_2 (`AddComponent|NODE_AddInstancedStaticMeshComponent-0`))
  (set `self.LadderSegmentInstances` _returnvalue_2)
  ;;[1 1 1] Loop ladder segment construction based on ladder height vector
  (for _index (range (+ (`KismetMathLibrary.FTrunc` (/ (.z (`self.LadderHeight`)) 50.0)) 1))
    ;;[1 1 1] Add a ladder segment instance
    (`InstancedStaticMeshComponent.AddInstance` (`self.LadderSegmentInstances`) (`KismetMathLibrary.MakeTransform` (`KismetMathLibrary.MakeVector` 0.0 0.0 (* _index 50.0)))))
  ;;[1 1 1] Rescale overlap box and center to ladder
  (`BoxComponent.SetBoxExtent` (`self.Box`) (`KismetMathLibrary.MakeVector` 25.0 25.0 _returnvalue) false)
  (`SceneComponent.K2_AddRelativeLocation` (`self.Box`) (`KismetMathLibrary.MakeVector` 0.0 0.0 _returnvalue) false false))