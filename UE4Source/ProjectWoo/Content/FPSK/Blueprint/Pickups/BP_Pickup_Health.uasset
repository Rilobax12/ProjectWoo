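; BP_Pickup_Health is a health pickup that restores a set amount of health to the character that collects it.
; Its PickupEffect event adds HealthRecoverAmount clamped to MaxHealth, then calls PickupEvent to hide the pickup and start its respawn timer.
; When health is already full, the pickup is not consumed and the character's HUD shows a short subtitle instead.
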(event `self.PickupEffect`
  (bind _characterreference (`self.CharacterReference`))
  (bind _characterreference_2 (`self.CharacterReference`))
  ;[0 0 0] Health pickup event
  (if (< (`/Game/FPSK/FirstPersonAssets/FirstPersonBP/Blueprints/FirstPersonCharacter.Health` _characterreference_2) (`/Game/FPSK/FirstPersonAssets/FirstPersonBP/Blueprints/FirstPersonCharacter.MaxHealth` _characterreference_2))
    ;;[1 1 1] Health recover
    (set `/Game/FPSK/FirstPersonAssets/FirstPersonBP/Blueprints/FirstPersonCharacter.Health` (`KismetMathLibrary.FClamp` (+ (`/Game/FPSK/FirstPersonAssets/FirstPersonBP/Blueprints/FirstPersonCharacter.Health` _characterreference) (`self.HealthRecoverAmount`)) 0.0 (`/Game/FPSK/FirstPersonAssets/FirstPersonBP/Blueprints/FirstPersonCharacter.MaxHealth` _characterreference)) (`self.CharacterReference`))
    ;;[1 1 1] Hide and Respawn timer events
    (`self.PickupEvent`)
    (else
      ;;[1 1 1] Play subtitle
      (`/Game/FPSK/Blueprint/Widget/BP_MainHUD.PlaySubtitle` (`/Game/FPSK/FirstPersonAssets/FirstPersonBP/Blueprints/FirstPersonCharacter.MainHUD` (`self.CharacterReference`)) "Health is already full." 2.0))))

(fn `UserConstructionScript`
  (`parent.UserConstructionScript`))